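; Interactive Rubik's cube puzzle of configurable dimensions that a nearby pawn can play or carry.
; Construction builds the cube meshes; BeginPlay spawns a BP_Rotator per slice to turn and randomize layers.
; Overlap and camera trace enable input; a physics handle holds the cube before the camera for mouse rotation.
; After turns it compares piece rotations; when solved, it animates the move-counter widget, spawns BP_Second_Buzzle and destroys itself.
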(event OnComponentBeginOverlap(PickUPCollsion)
  (params (OverlappedComponent :type Primitive%20Component%20Object%20Reference) (OtherActor :type Actor%20Object%20Reference) (OtherComp :type Primitive%20Component%20Object%20Reference) (OtherBodyIndex :type Integer) (bFromSweep :type Boolean) (SweepResult :type Hit%20Result%20Structure%20%28by%20ref%29))
  ;[1 1 1] Comment
  (if (not (Variables|Default|GetIn%20Use))
    (bind _aspawn (Utilities|Casting|CastToPawn OtherActor))
    (Variables|Default|SetColiding%20Pawn _aspawn)))

(event OnComponentEndOverlap(PickUPCollsion)
  (params (OverlappedComponent :type Primitive%20Component%20Object%20Reference) (OtherActor :type Actor%20Object%20Reference) (OtherComp :type Primitive%20Component%20Object%20Reference) (OtherBodyIndex :type Integer))
  ;[1 1 1] Comment
  (if (not (Utilities|Array|ContainsItem (Collision|GetOverlappingActors (Variables|Default|GetPickUP%20Collsion) 0 :!class /Script/Engine.PrimitiveComponent) (Variables|Default|GetColiding%20Pawn)))
    (CallFunction|StopPlaying)
    (Variables|Default|SetColiding%20Pawn 0)
    (if (Variables|Default|Get3D%20Widget)
      (Rendering|SetVisibility (Variables|Default|GetWidget) false false)
      (else
        (Widget|RemovefromParent (Variables|Default|GetWidget_Ref))))))

(event Custom|Toggle%20Play
  ;[1 1 1] Comment
  (if (Variables|Default|GetIn%20Use)
    (if (Variables|Default|GetPickUPCube)
      (CallFunction|StopPlaying)
      (CallFunction|Play)
      (else
        (CallFunction|StopPlaying)))
    (else
      (CallFunction|Play))))

(event Custom|Update%20Position
  (bind _coliding_pawn (Variables|Default|GetColiding%20Pawn))
  (bind _playerstate (Variables|/Script/Engine.Pawn|GetPlayerState _coliding_pawn))
  (bind _returnvalue (Game|GetPlayerController _playerstate))
  (bind _playercameramanager (Variables|/Script/Engine.PlayerController|GetPlayerCameraManager _returnvalue))
  ;[1 1 1] Comment
  (if (Variables|Default|GetIn%20Use)
    (Physics|Components|PhysicsHandle|SetTargetLocation (Variables|Default|GetHandle%20Component%20Ref) (+ (Camera|GetCameraLocation _playercameramanager) (/ (* (Math|Vector|GetForwardVector (Camera|GetCameraRotation _playercameramanager)) (Math|Vector|GetMaxElement (Transformation|GetActorScale3D)) (/ 1e+02 (Camera|GetFOVAngle _playercameramanager)) (Math|Float|SelectFloat (* (/ (Variables|/Script/Engine.SphereComponent|GetSphereRadius (Variables|Default|GetPickUP%20Collsion)) 3.0) (Variables|Default|GetHolding%20Distance%20Multiplier)) (Variables|Default|GetPlay%20Distance) (Variables|Default|GetPickUPCube)) (+ (/ (Math|Conversions|ToFloat(Integer) (+ (Variables|Default|GetCube%20X) (Variables|Default|GetCube%20Y) (Variables|Default|GetCube%20Z))) 6e+01) 1.0)) (Math|Float|Clamp(Float) (Class|WidgetLayoutLibrary|GetViewportScale) 0.6))))))

(event Custom|Trace
  (bind _coliding_pawn (Variables|Default|GetColiding%20Pawn))
  (bind _3d_widget (Variables|Default|Get3D%20Widget))
  (bind _widget_ref (Variables|Default|GetWidget_Ref))
  (bind _widget (Variables|Default|GetWidget))
  (bind _playerstate (Variables|/Script/Engine.Pawn|GetPlayerState _coliding_pawn))
  (bind _returnvalue (Game|GetPlayerController _playerstate))
  (bind _playercameramanager (Variables|/Script/Engine.PlayerController|GetPlayerCameraManager _returnvalue))
  (bind _returnvalue_2 (Camera|GetCameraLocation _playercameramanager))
  ;[1 1 1] Comment
  (if (not (Variables|Default|GetIn%20Use))
    (Utilities|IsValid _coliding_pawn
      (:Is%20Valid
        (bind _outhit (Collision|LineTraceByChannel _returnvalue_2 (+ _returnvalue_2 (* (Math|Vector|GetForwardVector (Camera|GetCameraRotation _playercameramanager)) (+ (Variables|Default|GetPick%20Up%20Radius) (Math|Vector|Distance2D(Vector) _returnvalue_2 (Transformation|GetActorLocation))) 2.0)) "TraceTypeQuery1" false (Utilities|Array|MakeArray _coliding_pawn) "ForOneFrame" false))
        (if (== (.HitActor (Collision|BreakHitResult _outhit)) self)
          (Utilities|FlowControl|Sequence
            (:then_0
              (Utilities|FlowControl|DoOnce false :!label _label
                (:Completed
                  (Variables|Default|SetHovering true)
                  (if _3d_widget
                    (Rendering|SetVisibility _widget true false)
                    (else
                      (UserInterface|Viewport|AddtoViewport _widget_ref 0))))))
            (:then_1
              (goto _label_2 Reset)))
          (else
            (Utilities|FlowControl|Sequence
              (:then_0
                (goto _label Reset))
              (:then_1
                (Utilities|FlowControl|DoOnce false :!label _label_2
                  (:Completed
                    (Variables|Default|SetHovering false)
                    (if _3d_widget
                      (Rendering|SetVisibility _widget false false)
                      (else
                        (Widget|RemovefromParent _widget_ref)))))))))))))

(event Custom|Toggle%20PickUP
  ;[1 1 1] Comment
  (if (Variables|Default|GetIn%20Use)
    (if (Variables|Default|GetPickUPCube)
      (CallFunction|StopPlaying)
      (else
        (CallFunction|StopPlaying)
        (CallFunction|PickUP)))
    (else
      (CallFunction|PickUP))))

(event Custom|Auto%20Randomize
  ;[1 1 1] Comment
  (CallFunction|StartRandomize)
  (Utilities|FlowControl|Delay 0.0)
  (CallFunction|StopRandomize)
  (Variables|Default|SetBegining%20Randomization false))

(event EventBeginPlay
  ;[1 1 1] Comment
  (Physics|SetEnableGravity (Variables|Default|GetCube%20Collision) (Variables|Default|GetGravity%20Enabled))
  (CallFunction|ConstructRotators)
  (Rendering|SetActorHiddenInGame (Variables|Default|GetRotators%20Ref) true)
  (bind _returnvalue (UserInterface|CreateWidget "/Game/Rubix_Cube_Project/Rubix_Cube/UI/Rubix_Widget.Rubix_Widget_C" 0 self))
  (bind _output_get (Variables|Default|SetWidget_Ref _returnvalue))
  (UserInterface|SetWidget (Variables|Default|GetWidget) _output_get)
  (for _array_element (Components|GetChildrenComponents (Variables|Default|GetCube%20Collision) false)
    (bind _asstatic_mesh_component (Utilities|Casting|CastToStaticMeshComponent _array_element))
    (Utilities|Array|AddUnique (Variables|Default|GetCubes%20Ref) _asstatic_mesh_component))
  (if (Variables|Default|GetBegining%20Randomization)
    (CallFunction|AutoRandomize)))

(event EventRotationStarted
  (Audio|PlaySoundatLocation (Variables|Default|GetClicked%20Sound) (Transformation|GetActorLocation) "0, 0, 0" 1.0 1.0 0.0 0 0 0 0)
  (bind _result (Math|Integer|IncrementInt (Variables|Default|GetMoves))
    (:%20%20
      (Default|UpdateCounter (Variables|Default|GetWidget_Ref) _result))))

(event EventPlay
  (bind _cube_collision (Variables|Default|GetCube%20Collision))
  (bind _pickupcube (Variables|Default|GetPickUPCube))
  (bind _coliding_pawn (Variables|Default|GetColiding%20Pawn))
  (bind _audio (Variables|Default|GetAudio))
  (bind _returnvalue (Transformation|GetWorldTransform _cube_collision))
  (bind _sound (Variables|/Script/Engine.AudioComponent|GetSound _audio))
  ;[1 1 1] Comment
  (if (not (Variables|Default|GetIn%20Use))
    (Variables|Default|SetIn%20Use true)
    (bind _returnvalue_2 (AddComponent|AddPhysicsHandleComponent (Game|Player|GetPlayerPawn 0)))
    (Variables|Default|SetHandle%20Component%20Ref _returnvalue_2)
    (Collision|SetCollisionResponsetoAllChannels _cube_collision "ECR_Ignore")
    (Physics|Components|PhysicsHandle|GrabComponentatLocationwithRotation (Variables|Default|GetHandle%20Component%20Ref) _cube_collision "None" (.location _returnvalue) (.rotation _returnvalue))
    (Utilities|StoreUserSettings)
    (Audio|PlaySoundatLocation (select _pickupcube "/Engine/VREditor/Sounds/UI/Object_PickUp.Object_PickUp" "/Game/Rubix_Cube_Project/Rubix_Cube/Audio/Hover.Hover") (.location _returnvalue) "0, 0, 0" 1.0 1.0 0.0 0 0 0 0)
    (Class|PhysicsHandleComponent|SetInterpolationSpeed (Variables|Default|GetHandle%20Component%20Ref) (Math|Float|SelectFloat 3e+01 6.0 _pickupcube))
    (if _pickupcube
      (Audio|Components|Audio|FadeOut (Variables|Default|GetAudio) 1.0 0.0 "Linear" :!class /Script/Engine.AudioComponent)
      (else
        (Rendering|SetActorHiddenInGame (Variables|Default|GetRotators%20Ref) false)
        (Utilities|SetUserSettings true true true)
        (Input|DisableInput _coliding_pawn (Game|GetPlayerController (Variables|/Script/Engine.Pawn|GetPlayerState _coliding_pawn)))
        (Utilities|IsValid _sound
          (:Is%20Valid
            (Audio|Components|Audio|FadeIn _audio 2.0 (Variables|Default|GetBackground%20Music%20Vol) (Math|Random|RandomFloatinRange 1.0 (/ (Variables|/Script/Engine.SoundBase|GetDuration _sound) 2.0)) "Linear" :!class /Script/Engine.AudioComponent)
            ;[1 1 1] Comment
            (bind _alpha (Timeline|Update%20View PlayFromStart)
              (:Update
                (bind _coliding_pawn_2 (Variables|Default|GetColiding%20Pawn)
                  (:then
                    (Pawn|SetControlRotation (Game|GetPlayerController (Variables|/Script/Engine.Pawn|GetPlayerState _coliding_pawn_2)) (Math|Rotator|Lerp(Rotator) (Pawn|GetControlRotation (Game|GetPlayerController (Variables|/Script/Engine.Pawn|GetPlayerState _coliding_pawn_2)) :!class /Script/Engine.Controller) (Math|Rotator|MakeRotator (.roll (Pawn|GetControlRotation (Game|GetPlayerController (Variables|/Script/Engine.Pawn|GetPlayerState _coliding_pawn_2)) :!class /Script/Engine.Controller)) 3.6e+02 (.yaw (Pawn|GetControlRotation (Game|GetPlayerController (Variables|/Script/Engine.Pawn|GetPlayerState _coliding_pawn_2)) :!class /Script/Engine.Controller))) _alpha true)))
                  (:else)))))
          (:Is%20Not%20Valid
            (Timeline|Update%20View PlayFromStart)))))))

(event EventStopPlaying
  (bind _coliding_pawn (Variables|Default|GetColiding%20Pawn))
  (bind _cube_collision (Variables|Default|GetCube%20Collision))
  ;[1 1 1] Comment
  (Variables|Default|GetColiding%20Pawn
    (:then
      (Variables|Default|SetPickUPCube false)
      (Variables|Default|SetIn%20Use false)
      (Rendering|SetActorHiddenInGame (Variables|Default|GetRotators%20Ref) true)
      (Utilities|SetUserSettings (Variables|Default|GetPrevious%20Show%20Mouse) (Variables|Default|GetPrevious%20Click%20Events) (Variables|Default|GetPrevious%20Mouse%20Over%20Events))
      (Collision|SetCollisionResponsetoChannel _cube_collision "ECC_WorldDynamic" "ECR_Block")
      (Collision|SetCollisionResponsetoChannel _cube_collision "ECC_WorldStatic" "ECR_Block")
      (Collision|SetCollisionResponsetoChannel _cube_collision "ECC_Visibility" "ECR_Block")
      (bind _handle_component_ref (Variables|Default|GetHandle%20Component%20Ref)
        (:then
          (Physics|Components|PhysicsHandle|ReleaseComponent _handle_component_ref)
          (Components|DestroyComponent _handle_component_ref))
        (:else
          _))
      (Input|EnableInput _coliding_pawn (Game|GetPlayerController (Variables|/Script/Engine.Pawn|GetPlayerState _coliding_pawn)))
      (Audio|Components|Audio|Stop (Variables|Default|GetUpdate%20View))
      (Audio|Components|Audio|FadeOut (Variables|Default|GetAudio) 1.0 0.0 "Linear" :!class /Script/Engine.AudioComponent))
    (:else)))

(event EventPickUP
  ;[1 1 1] Comment
  (Variables|Default|SetPickUPCube true)
  (CallFunction|Play))

(event EventStartRandomize
  ;[1 1 1] Input Actions and Randomization
  (if (CallFunction|IsRotating)
    (Development|PrintString "Can not While Rotating")
    (else
      (Class|RubixCubeInterface|UpdateRotatorSettings(Message) (Variables|Default|GetRotators%20Ref) (/ 1.0 (Variables|Default|GetRandomize%20Speed)))
      (Utilities|FlowControl|Sequence
        (:then_0
          (goto _label_2 Open))
        (:then_1
          (Class|RubixCubeInterface|TryRotateChildren(Message) (.OutItem (Utilities|Array|Random (Variables|Default|GetRotators%20Ref))) (Math|Random|RandomBool) :!label _label)
          (Utilities|FlowControl|Delay (+ (Variables|Default|GetRandomize%20Speed) 0.01))
          (Utilities|FlowControl|Gate true :!label _label_2
            (:Exit
              (if (Variables|Default|GetIn%20Use)
                (goto _label)
                (elif (Variables|Default|GetBegining%20Randomization)
                  (goto _label)
                  (else
                    (CallFunction|StopRandomize)))))))))))

(event EventStopRandomize
  ;[1 1 1] Input Actions and Randomization
  (Class|RubixCubeInterface|UpdateRotatorSettings(Message) (Variables|Default|GetRotators%20Ref) (Variables|Default|GetRotation%20speed))
  (Utilities|FlowControl|Gate true) ; enters at Close
)

(event EventTick
  (params (DeltaSeconds :type Float%20%28single-precision%29))
  ;[1 1 1] Comment
  (Variables|Default|GetColiding%20Pawn
    (:then
      (CallFunction|UpdatePosition)
      (CallFunction|Trace))
    (:else)))

(event EventRotationEnded
  (bind _widget_ref (Variables|Default|GetWidget_Ref))
  (if (CallFunction|GetState)
    (if (Variables|Default|GetBegining%20Randomization)
      (Variables|Default|SetBegining%20Randomization true)
      (CallFunction|AutoRandomize)
      (else
        (Audio|PlaySoundatLocation "/Engine/VREditor/Sounds/UI/Click_on_Button.Click_on_Button" (Transformation|GetActorLocation) "0, 0, 0" 1.0 1.0 0.0 0 0 0 0)
        (Default|SolvedAnim _widget_ref)
        (bind _output_get (Variables|Default|SetMoves 0))
        (Default|UpdateCounter _widget_ref _output_get)
        (Utilities|FlowControl|Delay 0.5)
        (Game|SpawnActorfromClass "/Game/BP_Second_Buzzle.BP_Second_Buzzle_C" (Math|Transform|MakeTransform (Transformation|GetActorLocation) "0, 0, 0" "1.000000,1.000000,1.000000") "Undefined" "MultiplyWithRoot" 0 0)
        (Actor|DestroyActor)))))

(event EventResetCube
  ;[1 1 1] Input Actions and Randomization
  (if (CallFunction|IsRotating)
    (Development|PrintString "Can not While Rotating")
    (else
      (Transformation|SetRelativeRotation (Variables|Default|GetCubes%20Ref) "0, 0, 0" false false)
      (bind _output_get (Variables|Default|SetMoves 0))
      (Default|UpdateCounter (Variables|Default|GetWidget_Ref) _output_get))))

(event MouseInput|EventActorOnClicked
  (params (ButtonPressed :type Key%20Structure :default "None"))
  ;[1 1 1] Comment
  (if (Variables|Default|GetIn%20Use)
    _))

(event EventActorOnReleased
  (params (ButtonReleased :type Key%20Structure :default "None"))
  ;[1 1 1] Comment
  (if (Variables|Default|GetIn%20Use)
    _))

(event MouseInput|EventActorBeginCursorOver
  ;[1 1 1] Comment
)

(event MouseInput|EventActorEndCursorOver
  ;[1 1 1] Comment
)

(event Input|KeyboardEvents|F
  (params (Key :type Key%20Structure :default "None"))
  ;[1 1 1] Input Actions and Randomization
  (:Pressed
    (if (Variables|Default|GetHovering)
      (CallFunction|TogglePlay))))

(event Input|KeyboardEvents|R
  (params (Key :type Key%20Structure :default "None"))
  (bind _handle_component_ref (Variables|Default|GetHandle%20Component%20Ref))
  ;[1 1 1] Input Actions and Randomization
  (:Released
    (if (and (Variables|Default|GetIn%20Use) (Utilities|IsValid _handle_component_ref))
      (Default|StopReset (Variables|Default|GetWidget_Ref))
      (Class|PhysicsHandleComponent|SetTargetRotation _handle_component_ref (Math|Rotator|FindLookatRotation (Transformation|GetWorldLocation (Variables|Default|GetCube%20Collision)) (Camera|GetCameraLocation (Game|GetPlayerCameraManager 0)))))))

(event Input|MouseEvents|LeftMouseButton
  (params (Key :type Key%20Structure :default "None"))
  (bind _returnvalue (Game|GetPlayerCameraManager 0))
  (bind _returnvalue_2 (Transformation|GetActorRotation _returnvalue))
  ;[1 1 1] Comment
  (:Pressed
    (if (Variables|Default|GetIn%20Use)
      (Utilities|FlowControl|Gate true) ; enters at Open
    ))
  (:Released
    (Utilities|FlowControl|Gate true) ; enters at Close
  ))

(event Input|KeyboardEvents|G
  (params (Key :type Key%20Structure :default "None"))
  (bind _widget_ref (Variables|Default|GetWidget_Ref))
  ;[1 1 1] Input Actions and Randomization
  (:Pressed
    (if (Variables|Default|GetIn%20Use)
      (Default|StartRandomize _widget_ref (/ 1.0 (Variables|Default|GetHold%20Time)))))
  (:Released
    (if (Variables|Default|GetIn%20Use)
      (Default|StopRandomize _widget_ref)
      (CallFunction|StopRandomize)
      (bind _output_get (Variables|Default|SetMoves 0))
      (Default|UpdateCounter (Variables|Default|GetWidget_Ref) _output_get))))

(event Input|KeyboardEvents|E
  (params (Key :type Key%20Structure :default "None"))
  ;[1 1 1] Input Actions and Randomization
  (:Pressed
    (if (Variables|Default|GetHovering)
      (CallFunction|TogglePickUP))))

(event Input|MouseEvents|Mouse2D
  (params (AxisValue :type Vector :default "0, 0, 0"))
  (bind _returnvalue (Game|GetPlayerCameraManager 0))
  (bind _returnvalue_2 (Transformation|GetActorRotation _returnvalue))
  ;[1 1 1] Comment
  (Utilities|FlowControl|Gate true
    (:Exit
      (Class|PhysicsHandleComponent|SetTargetRotation (Variables|Default|GetHandle%20Component%20Ref) (Math|Rotator|CombineRotators (Transformation|GetActorRotation) (* (Math|Rotator|CombineRotators (Math|Vector|RotatorfromAxisandAngle (Math|Vector|GetUpVector _returnvalue_2) (* (.x AxisValue) -1.0)) (Math|Vector|RotatorfromAxisandAngle (Math|Vector|GetRightVector _returnvalue_2) (.y AxisValue))) (Variables|Default|GetRotation%20Sensetivity)))))))

(fn ConstructionScript
  ;[1 1 1] Comment
  (Components|Box|SetBoxExtent (Variables|Default|GetCube%20Collision) (Math|Vector|MakeVector (Math|Conversions|ToFloat(Integer) (Variables|Default|GetCube%20X)) (Math|Conversions|ToFloat(Integer) (Variables|Default|GetCube%20Y)) (Math|Conversions|ToFloat(Integer) (Variables|Default|GetCube%20Z))) true)
  ;[1 1 1] Comment
  (CallFunction|ConstructCube)
  ;[1 1 1] Comment
  (Components|Sphere|SetSphereRadius (Variables|Default|GetPickUP%20Collsion) (Variables|Default|GetPick%20Up%20Radius) true)
  (if (not (Variables|Default|GetScale%20Radius%20With%20Object))
    (Transformation|SetWorldScale3D (Variables|Default|GetPickUP%20Collsion) "1.000000,1.000000,1.000000")
    (Audio|Components|Audio|SetSound (Variables|Default|GetAudio) (Variables|Default|GetBackground%20Music))))

(fn GetState
  (for _array_element (Variables|Default|GetCubes%20Ref)
    (Utilities|FlowControl|Sequence
      (:then_0
        (Utilities|FlowControl|DoOnce false
          (:Completed
            (LocalVariables|SetInitial%20Rot (Transformation|GetWorldRotation _array_element)))))
      (:then_1
        (if (Utilities|Operators|EqualEqual (LocalVariables|GetInitial%20Rot) (Transformation|GetWorldRotation _array_element) 1.0)
          (LocalVariables|SetSolve_State true)
          (else
            (bind _output_get (LocalVariables|SetSolve_State false))
            (return _output_get))))))
  (return (LocalVariables|GetSolve_State)))

(fn IsRotating
  (for _array_element (Variables|Default|GetRotators%20Ref)
    (if (Variables|/Game/Rubix_Cube_Project/Rubix_Cube/Blueprint/BP_Rotator.BP_Rotator_C|GetAttached _array_element)
      (return true)))
  (return false))

(fn ConstructCube
  (bind _cube_mesh_radius (Variables|Default|GetCube_Mesh_Radius))
  ;[1 1 1] Comment
  (for _index (range 1 (Variables|Default|GetCube%20X))
    (for _index_2 (range 1 (Variables|Default|GetCube%20Y))
      (for _index_3 (range 1 (Variables|Default|GetCube%20Z))
        (bind _returnvalue (AddComponent|AddStaticMeshComponent true (Math|Transform|MakeTransform (+ (- (Math|Vector|MakeVector (* (- _index 1) _cube_mesh_radius) (* (- _index_2 1) _cube_mesh_radius) (* (- _index_3 1) _cube_mesh_radius)) (Variables|/Script/Engine.BoxComponent|GetBoxExtent (Variables|Default|GetCube%20Collision))) (/ (Variables|Default|GetCube_Mesh_Radius) 2.0)) "0, 0, 0" "1.000000,1.000000,1.000000")))
        (Transformation|AttachComponentToComponent _returnvalue (Variables|Default|GetCube%20Collision) "None" "KeepRelative" "KeepRelative" "KeepRelative" true)
        (Components|StaticMesh|SetStaticMesh _returnvalue (Variables|Default|GetCube%20Style))))))

(fn ConstructRotators
  (bind _button_style (Variables|Default|GetButton%20Style))
  (bind _rotation_speed (Variables|Default|GetRotation%20speed))
  (bind _cube_x (Variables|Default|GetCube%20X))
  (bind _cube_collision (Variables|Default|GetCube%20Collision))
  (bind _rotators_ref (Variables|Default|GetRotators%20Ref))
  (bind _cube_mesh_radius (Variables|Default|GetCube_Mesh_Radius))
  (bind _rotators (Variables|Default|GetRotators))
  (bind _cube_y (Variables|Default|GetCube%20Y))
  (bind _cube_z (Variables|Default|GetCube%20Z))
  (bind _returnvalue (/ _cube_mesh_radius 4.0))
  (bind _boxextent (Variables|/Script/Engine.BoxComponent|GetBoxExtent _cube_collision))
  ;[1 1 1] Comment
  (for _index (range 1 _cube_x)
    (bind _returnvalue_2 (Game|SpawnActorfromClass "/Game/Rubix_Cube_Project/Rubix_Cube/Blueprint/BP_Rotator.BP_Rotator_C" (Math|Transform|MakeTransform (Math|Vector|MakeVector (Utilities|Operators|Subtract (* _index _cube_mesh_radius) (/ _cube_mesh_radius 2.0) _cube_x) 0.0 0.0) "0.000000,90.000000,-90.000000" "1.000000,1.000000,1.000000") "AlwaysSpawn" "MultiplyWithRoot" 0 (Math|Vector|MakeVector (.y _boxextent) (.z _boxextent) _returnvalue) _rotation_speed _button_style 0))
    (Transformation|AttachComponentToComponent _returnvalue_2 _rotators "None" "KeepRelative" "KeepRelative" "KeepRelative" true)
    (Utilities|Array|AddUnique _rotators_ref _returnvalue_2))
  (for _index_2 (range 1 _cube_y)
    (bind _returnvalue_3 (Game|SpawnActorfromClass "/Game/Rubix_Cube_Project/Rubix_Cube/Blueprint/BP_Rotator.BP_Rotator_C" (Math|Transform|MakeTransform (Math|Vector|MakeVector 0.0 (Utilities|Operators|Subtract (* _index_2 _cube_mesh_radius) (/ _cube_mesh_radius 2.0) _cube_y) 0.0) "90.000000,-90.000000,0.000000" "1.000000,1.000000,1.000000") "AlwaysSpawn" "MultiplyWithRoot" 0 (Math|Vector|MakeVector (.z _boxextent) (.x _boxextent) _returnvalue) _rotation_speed _button_style 0))
    (Transformation|AttachComponentToComponent _returnvalue_3 _rotators "None" "KeepRelative" "KeepRelative" "KeepRelative" true)
    (Utilities|Array|AddUnique _rotators_ref _returnvalue_3))
  (for _index_3 (range 1 _cube_z)
    (bind _returnvalue_4 (Game|SpawnActorfromClass "/Game/Rubix_Cube_Project/Rubix_Cube/Blueprint/BP_Rotator.BP_Rotator_C" (Math|Transform|MakeTransform (Math|Vector|MakeVector 0.0 0.0 (Utilities|Operators|Subtract (* _index_3 _cube_mesh_radius) (/ _cube_mesh_radius 2.0) _cube_z)) "0.000000,-90.000000,-0.000000" "1.000000,1.000000,1.000000") "AlwaysSpawn" "MultiplyWithRoot" 0 (Math|Vector|MakeVector (.y _boxextent) (.x _boxextent) _returnvalue) _rotation_speed _button_style 0))
    (Transformation|AttachComponentToComponent _returnvalue_4 _rotators "None" "KeepRelative" "KeepRelative" "KeepRelative" true)
    (Utilities|Array|AddUnique _rotators_ref _returnvalue_4)))